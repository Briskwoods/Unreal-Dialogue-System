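; NPC that shows data-table dialogue in a UI widget and toggles the player's interaction prompt through box overlaps.
; At BeginPlay it gathers the Dialogue row names matching its NPCID.
; Each Interact increments the line counter and adds a new widget showing the row that matches ConversationID and that line.
; Without exactly one match, the newly created widget is removed and the counter resets.
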(event `self.ReceiveBeginPlay`
  (bind _outrownames (`DataTableFunctionLibrary.GetDataTableRowNames` "/Game/Dialogue/Dialogue.Dialogue"))
  (for _array_element _outrownames
    (bind _returnvalue (`|GetDataTableRow` "/Game/Dialogue/Dialogue.Dialogue" _array_element)
      (:`then`
        (if (== (`.NPC_ID_2_3F3913114CB6F04FF58D9785EBFD8630` (break `/Game/Dialogue/DialogueStructure` _returnvalue)) (`self.NPC_ID`))
          (`KismetArrayLibrary.Array_Add` (`self.Dialogue`) _array_element))))))

(event `/Game/Blueprints/InteractPrompt_I.Interact`
  (`/Engine/EditorBlueprintResources/StandardMacros.IncrementInt` (`self.LineCurrent`)
    (:`  `
      (`self.CreateDialogue`))))

(event `self.Box.OnComponentBeginOverlap`
  (params (OverlappedComponent :type "PrimitiveComponent Object Reference") (OtherActor :type "Actor Object Reference") (OtherComp :type "PrimitiveComponent Object Reference") (OtherBodyIndex :type Integer) (bFromSweep :type Boolean) (SweepResult :type "HitResult Structure (by ref)"))
  ;[1 1 1] Interaction Prompt
  (if (`self.ActorHasTag` OtherActor "Player")
    (message `/Game/Blueprints/BPI_PlayerManagement.Show Interaction Prompt` OtherActor)
    (message `/Game/Blueprints/BPI_PlayerManagement.Set Interaction State` OtherActor true)))

(event `self.Box.OnComponentEndOverlap`
  (params (OverlappedComponent :type "PrimitiveComponent Object Reference") (OtherActor :type "Actor Object Reference") (OtherComp :type "PrimitiveComponent Object Reference") (OtherBodyIndex :type Integer))
  ;[1 1 1] Interaction Prompt
  (if (`self.ActorHasTag` OtherActor "Player")
    (message `/Game/Blueprints/BPI_PlayerManagement.Hide Interaction Prompt` OtherActor)
    (message `/Game/Blueprints/BPI_PlayerManagement.Set Interaction State` OtherActor false)))

(fn `CreateDialogue`
  (bind _dialoguewidget (`self.DialogueWidget`))
  (bind _returnvalue (`|CreateWidget` "/Game/Dialogue/DialogueWidget.DialogueWidget_C" (`GameplayStatics.GetPlayerController` 0)))
  (bind _output_get (set `self.DialogueWidget` _returnvalue))
  (`UserWidget.AddToViewport` _output_get 0)
  (bind _returned_line (`self.GetDialogueLine`))
  (`/Engine/EditorBlueprintResources/StandardMacros.IsValid` _dialoguewidget
    (:`Is Valid`
      (set `/Game/Dialogue/DialogueWidget.DialogueText` _returned_line _dialoguewidget))))

(fn `GetDialogueLine`
  (returns (`Returned Line` :type Text))
  (locals (returnedLines :type "Array of Text"))
  (for _array_element (`self.Dialogue`)
    (bind _returnvalue (`|GetDataTableRow` "/Game/Dialogue/Dialogue.Dialogue" _array_element)
      (:`then`
        (bind (_npc_id _conversation_id _line_id _dialogue) (break `/Game/Dialogue/DialogueStructure` _returnvalue))
        (if (and (== _conversation_id (`self.Conversation_ID`)) (== _line_id (`self.LineCurrent`)))
          (`KismetArrayLibrary.Array_Add` (`local.returnedLines`) _dialogue)))))
  (if (== (`KismetArrayLibrary.Array_Length` (`local.returnedLines`)) 1)
    (return (`|GetArrayItem` (`local.returnedLines`)))
    (else
      (`Widget.RemoveFromParent` (`self.DialogueWidget`))
      (set `self.DialogueWidget` null)
      (set `self.LineCurrent` 0))))

(fn `UserConstructionScript`)