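; Interactible actor that gives the player an interaction prompt and a toggleable dialogue box.
; A Box overlap with an actor tagged "Player" sends it messages to show or hide the prompt and set its interaction state.
; The Interact event removes an existing dialogue widget, or creates one, adds it to the viewport and fills it with the actor's MyText.
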(event `/Game/Blueprints/InteractPrompt_I.Interact`
  ;[1 1 1] Dialogue Interact Functionality
  (`/Engine/EditorBlueprintResources/StandardMacros.IsValid` (`self.DialogueWidget`)
    (:`Is Valid`
      (`Widget.RemoveFromParent` (`self.DialogueWidget`))
      (set `self.DialogueWidget` null))
    (:`Is Not Valid`
      (bind _returnvalue (`|CreateWidget` "/Game/Dialogue/DialogueWidget.DialogueWidget_C" (`GameplayStatics.GetPlayerController` 0)))
      (bind _output_get (set `self.DialogueWidget` _returnvalue))
      (`UserWidget.AddToViewport` _output_get 0)
      (set `/Game/Dialogue/DialogueWidget.DialogueText` (`self.MyText`) (`self.DialogueWidget`)))))

(event `self.Box.OnComponentBeginOverlap`
  (params (OverlappedComponent :type "PrimitiveComponent Object Reference") (OtherActor :type "Actor Object Reference") (OtherComp :type "PrimitiveComponent Object Reference") (OtherBodyIndex :type Integer) (bFromSweep :type Boolean) (SweepResult :type "HitResult Structure (by ref)"))
  ;[1 1 1] Interaction Prompt
  (if (`self.ActorHasTag` OtherActor "Player")
    (message `/Game/Blueprints/BPI_PlayerManagement.Show Interaction Prompt` OtherActor)
    (message `/Game/Blueprints/BPI_PlayerManagement.Set Interaction State` OtherActor true)))

(event `self.Box.OnComponentEndOverlap`
  (params (OverlappedComponent :type "PrimitiveComponent Object Reference") (OtherActor :type "Actor Object Reference") (OtherComp :type "PrimitiveComponent Object Reference") (OtherBodyIndex :type Integer))
  ;[1 1 1] Interaction Prompt
  (if (`self.ActorHasTag` OtherActor "Player")
    (message `/Game/Blueprints/BPI_PlayerManagement.Hide Interaction Prompt` OtherActor)
    (message `/Game/Blueprints/BPI_PlayerManagement.Set Interaction State` OtherActor false)))

(fn `UserConstructionScript`)